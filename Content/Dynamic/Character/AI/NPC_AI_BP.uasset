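; NPC_AI_BP is an AI controller for guard NPCs that react to perceived targets.
; On BeginPlay it sets up the Patrol_Data blackboard and runs the Guard_Behaviour behavior tree.
; When perception senses an actor not tagged "Enemy", it stores it as "Aiming Actor" and makes the controlled Character_BP aim and fire.
; Losing that stimulus clears the key and stops aiming and firing.
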(event OnTargetPerceptionUpdated(AIPerception)
  (params (Actor :type Actor%20Object%20Reference) (Stimulus :type AI%20Stimulus%20Structure))
  (if (not (Actor|ActorHasTag Actor "Enemy"))
    (if (.bSuccessfullySensed (Utilities|Struct|BreakAIStimulus Stimulus))
      (AI|Components|Blackboard|SetValueasObject (Variables|Default|GetBlackboard%20Component) (Utilities|String|StringToName "Aiming Actor") Actor)
      (bind _ascharacter_bp (Utilities|Casting|CastToCharacter_BP (Pawn|GetControlledPawn)))
      (Variables|/Game/Dynamic/Character/Behaviour/Character_BP.Character_BP_C|SetAiming _ascharacter_bp true)
      (Variables|/Game/Dynamic/Character/Behaviour/Character_BP.Character_BP_C|SetFiring _ascharacter_bp true)
      (else
        (AI|Components|Blackboard|ClearValue (Variables|Default|GetBlackboard%20Component) (Utilities|String|StringToName "Aiming Actor"))
        (bind _ascharacter_bp_2 (Utilities|Casting|CastToCharacter_BP (Pawn|GetControlledPawn)))
        (Variables|/Game/Dynamic/Character/Behaviour/Character_BP.Character_BP_C|SetAiming _ascharacter_bp_2 false)
        (Variables|/Game/Dynamic/Character/Behaviour/Character_BP.Character_BP_C|SetFiring _ascharacter_bp_2 false)))))

(event EventBeginPlay
  (bind _blackboardcomponent (Class|AIController|UseBlackboard "/Game/Dynamic/Character/AI/Patrol_Data.Patrol_Data"))
  (Variables|Default|SetBlackboard%20Component _blackboardcomponent)
  (AI|RunBehaviorTree "/Game/Dynamic/Character/AI/Guard_Behaviour.Guard_Behaviour"))

(fn ConstructionScript)