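; BP_FireComponent is a weapon behaviour scene component that fires ball projectiles with a rate limit.
; Tick accumulates the time since the last shot into LastFireTime.
; Fire spawns a BP_BallProjectile at the component's world transform and resets that timer, but only once the accumulated time reaches FireDelay.
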(event EventBeginPlay)

(event EventTick
  (params (DeltaSeconds :type Float%20%28single-precision%29))
  (Variables|Default|SetLast%20Fire%20Time (+ DeltaSeconds (Variables|Default|GetLast%20Fire%20Time))))

(fn Fire
  (if (>= (Variables|Default|GetLast%20Fire%20Time) (Variables|Default|GetFire%20Delay))
    (Variables|Default|SetLast%20Fire%20Time 0.0)
    (Game|SpawnActorfromClass "/Game/Dynamic/Weapons/FPWeapon/Behaviour/BP_BallProjectile.BP_BallProjectile_C" (Transformation|GetWorldTransform) "Undefined" 0 0)))