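; Terrain tile Blueprint with a barrier and an attach point.
; When the player character starts overlapping the Box trigger, the Barrier's collision is disabled; when the overlap ends, it is re-enabled for query and physics.
; An IsPlayerActor check filters both overlap events to the first player's character.
; GetAttachPoint exposes the AttachLocation world transform.
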(event OnComponentEndOverlap(Box)
  (params (OverlappedComponent :type Primitive%20Component%20Object%20Reference) (OtherActor :type Actor%20Object%20Reference) (OtherComp :type Primitive%20Component%20Object%20Reference) (OtherBodyIndex :type Integer))
  (Utilities|IsPlayerActor OtherActor)
  (CallFunction|SetLockBarrier true))

(event OnComponentBeginOverlap(Box)
  (params (OverlappedComponent :type Primitive%20Component%20Object%20Reference) (OtherActor :type Actor%20Object%20Reference) (OtherComp :type Primitive%20Component%20Object%20Reference) (OtherBodyIndex :type Integer) (bFromSweep :type Boolean) (SweepResult :type Hit%20Result%20Structure%20%28by%20ref%29))
  (Utilities|IsPlayerActor OtherActor)
  (CallFunction|SetLockBarrier false))

(fn ConstructionScript)

(fn GetAttachPoint
  (return (Transformation|GetWorldTransform (Variables|Default|GetAttach%20Location))))

(fn SetLockBarrier
  (params (Locked :type Boolean))
  (if Locked
    (Collision|SetCollisionEnabled (Variables|Default|GetBarrier) "QueryAndPhysics")
    (else
      (Collision|SetCollisionEnabled (Variables|Default|GetBarrier) "NoCollision"))))