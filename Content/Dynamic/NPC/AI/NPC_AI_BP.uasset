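; AI controller for guard NPCs that aim and fire at actors they perceive.
; On BeginPlay it sets up the Patrol_Data blackboard and runs the Guard_Behaviour tree.
; Perception updates for actors without the Enemy tag set or clear the Aiming Actor key and toggle Aiming and Firing on the controlled Ue4ASP_Character.
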(event OnTargetPerceptionUpdated(AIPerception)
  (params (Actor :type Actor%20Object%20Reference) (Stimulus :type AI%20Stimulus%20Structure))
  (if (not (Actor|ActorHasTag Actor "Enemy"))
    (if (.bSuccessfullySensed (Utilities|Struct|BreakAIStimulus Stimulus))
      (AI|Components|Blackboard|SetValueasObject (Variables|Default|GetBlackboard%20Component) (Utilities|String|StringToName "Aiming Actor") Actor)
      (bind _asue_4asp_character (Utilities|Casting|CastToUe4ASP_Character (Pawn|GetControlledPawn)))
      (Variables|/Game/Dynamic/NPC/Behaviour/Ue4ASP_Character.Ue4ASP_Character_C|SetAiming _asue_4asp_character true)
      (Variables|/Game/Dynamic/NPC/Behaviour/Ue4ASP_Character.Ue4ASP_Character_C|SetFiring _asue_4asp_character true)
      (else
        (AI|Components|Blackboard|ClearValue (Variables|Default|GetBlackboard%20Component) (Utilities|String|StringToName "Aiming Actor"))
        (bind _asue_4asp_character_2 (Utilities|Casting|CastToUe4ASP_Character (Pawn|GetControlledPawn)))
        (Variables|/Game/Dynamic/NPC/Behaviour/Ue4ASP_Character.Ue4ASP_Character_C|SetAiming _asue_4asp_character_2 false)
        (Variables|/Game/Dynamic/NPC/Behaviour/Ue4ASP_Character.Ue4ASP_Character_C|SetFiring _asue_4asp_character_2 false)))))

(event EventBeginPlay
  (bind _blackboardcomponent (Class|AIController|UseBlackboard "/Game/Dynamic/NPC/AI/Patrol_Data.Patrol_Data"))
  (Variables|Default|SetBlackboard%20Component _blackboardcomponent)
  (AI|RunBehaviorTree "/Game/Dynamic/NPC/AI/Guard_Behaviour.Guard_Behaviour"))

(fn ConstructionScript)